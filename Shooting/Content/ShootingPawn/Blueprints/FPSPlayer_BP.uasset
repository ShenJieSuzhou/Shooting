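; First-person shooter player Blueprint that handles aim-down-sights, the AWP scope and hit feedback.
; Holding right mouse with a gun runs timelines that blend camera FOV and arms-mesh transform, with tighter zoom for the AWP.
; The AWP also shows a scope widget created at BeginPlay and hides camera and mesh once zoomed.
; UnderAttack animates a vignette through a Material Parameter Collection, and a test event line-traces to spawn decals.
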(event `self.ReceiveBeginPlay`
  (bind _returnvalue (`|CreateWidget` "/Game/ShootingPawn/Blueprints/Scope_HUD.Scope_HUD_C"))
  (set `self.ScopeHUD` _returnvalue))

(event `UnderAttack`
  (bind (_direction _float) (`Timeline|Vignette` :!via `PlayFromStart`)
    (:`Update`
      (`KismetMaterialLibrary.SetScalarParameterValue` "/Game/ShootingPawn/Materials/FPSMaterial_MPC.FPSMaterial_MPC" "VignetteAmount" _float))))

(event `Key|RightMouseButton`
  (params (Key :type "Key Structure"))
  (bind _firstpersoncameracomponent (`self.FirstPersonCameraComponent`))
  (:`Pressed`
    (if (not (or (`|EnumEquality` (`self.CurWeaponType`) "EW_None") (`|EnumEquality` (`self.CurWeaponType`) "EW_Knife")))
      (if (`|EnumEquality` (`self.CurWeaponType`) "EW_AWP")
        (`UserWidget.AddToViewport` (`self.ScopeHUD`) 0))
      (`self.OnAimDownSight`)
      (bind (_direction _float) (`Timeline|Timeline_0` :!via `PlayFromStart`)
        (:`Update`
          (if (`|EnumEquality` (`self.CurWeaponType`) "EW_AWP")
            (set `self.ADSDistance` 30.0)
            (else
              (set `self.ADSDistance` 60.0)))
          (`CameraComponent.SetFieldOfView` _firstpersoncameracomponent (`KismetMathLibrary.Lerp` 90.0 (`self.ADSDistance`) _float))
          (`SceneComponent.K2_SetRelativeTransform` (`self.Mesh1P`) (`KismetMathLibrary.MakeTransform` (`KismetMathLibrary.VLerp` (3.177 -1.02 -23.0) (3.177 0.0 -16.0) _float) (struct :`Yaw` -1.0)) false false))
        (:`Finished`
          (bind _result (`self.IsSniper`))
          (if _result
            (`SceneComponent.SetVisibility` _firstpersoncameracomponent false false)
            (`SceneComponent.SetVisibility` (`self.Mesh1P`) false false))))))
  (:`Released`
    (if (not (or (`|EnumEquality` (`self.CurWeaponType`) "EW_None") (`|EnumEquality` (`self.CurWeaponType`) "EW_Knife")))
      (bind _result_2 (`self.IsSniper`))
      (if _result_2
        (`Widget.RemoveFromParent` (`self.ScopeHUD`))
        (`SceneComponent.SetVisibility` (`self.FirstPersonCameraComponent`) true false)
        (`SceneComponent.SetVisibility` (`self.Mesh1P`) true false))
      (`self.OnRecoverAimDownSight`)
      (bind (_direction_2 _float_2) (`Timeline|Timeline_1` :!via `PlayFromStart`)
        (:`Update`
          (`CameraComponent.SetFieldOfView` (`self.FirstPersonCameraComponent`) (`KismetMathLibrary.Lerp` (`self.ADSDistance`) 90.0 _float_2))
          (`SceneComponent.K2_SetRelativeTransform` (`self.Mesh1P`) (`KismetMathLibrary.MakeTransform` (`KismetMathLibrary.VLerp` (3.177 0.0 -16.0) (3.177 -1.02 -23.0) _float_2) (struct :`Yaw` 4.0)) false false))))))

(event `self.testSpawnDecal`
  (bind _firstpersoncameracomponent (`self.FirstPersonCameraComponent`))
  (bind (_outhit _returnvalue) (`KismetSystemLibrary.LineTraceSingle` (`SceneComponent.K2_GetComponentLocation` _firstpersoncameracomponent) (* (`SceneComponent.GetForwardVector` _firstpersoncameracomponent) 20000.0) "TraceTypeQuery1"))
  (if _returnvalue
    (`GameplayStatics.SpawnDecalAtLocation` "/Game/UWC_Bullet_Holes/Materials/M_Master_Normal.M_Master_Normal" (12.0 12.0 12.0) (`.Location` (`GameplayStatics.BreakHitResult` _outhit)) (`KismetMathLibrary.MakeRotFromX` (`.Normal` (`GameplayStatics.BreakHitResult` _outhit))))))

(fn `IsSniper`
  (returns (result :type Boolean))
  (if (`|EnumEquality` (`self.CurWeaponType`) "EW_AWP")
    (return true)
    (else
      (return false))))

(fn `UserConstructionScript`)