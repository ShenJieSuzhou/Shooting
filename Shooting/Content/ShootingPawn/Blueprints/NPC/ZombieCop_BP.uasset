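; Zombie cop NPC that wanders randomly until damage, sight or sound of the player sets it chasing.
; AIMoveTo callbacks loop the wander with random pauses, while PawnSensing and PointDamage trigger a faster chase targeting the player controller, not its pawn.
; AttackPlayer is a stub that only restarts the chase.
; Lethal point damage flags it dead, stops movement and destroys it after a random delay.
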(event `self.ReceiveBeginPlay`
  (`parent.ReceiveBeginPlay`)
  (set `self.CurrentHealth` (`self.MaxHealth`))
  (`self.AIMovement`))

(event `AIMovement`
  (if (not (`self.IsDead`))
    (`|AIMoveTo` self (`NavigationSystemV1.K2_GetRandomReachablePointInRadius` (`self.K2_GetActorLocation`) 5000.0 null null) null
      (:`OnSuccess`
        (`KismetSystemLibrary.Delay` (`KismetMathLibrary.RandomFloatInRange` 2.0 4.0) :!label _label)
        (`self.AIMovement`))
      (:`OnFail`
        (if (`self.IsDead`)
          _
          (elif (not (`self.IsActive`))
            (goto _label)))))))

(event `self.ReceivePointDamage`
  (params (Damage :type "Float (single-precision)") (DamageType :type "DamageType Object Reference") (HitLocation :type "Vector Structure") (HitNormal :type "Vector Structure") (HitComponent :type "PrimitiveComponent Object Reference") (BoneName :type Name) (ShotFromDirection :type "Vector Structure") (InstigatedBy :type "Controller Object Reference") (DamageCauser :type "Actor Object Reference") (HitInfo :type "HitResult Structure (by ref)"))
  (set `self.CurrentHealth` (- (`self.CurrentHealth`) Damage))
  (if (<= (`self.CurrentHealth`) 0.0)
    (set `self.IsDead` true)
    (`MovementComponent.StopMovementImmediately` (`self.CharacterMovement`))
    (`KismetSystemLibrary.Delay` (`KismetMathLibrary.RandomFloatInRange` 5.0 10.0))
    (`self.K2_DestroyActor`)
    (else
      (set `self.IsActive` true)
      (`self.HunterPlayer`))))

(event `HunterPlayer`
  (if (not (`self.IsDead`))
    (set `CharacterMovementComponent.MaxWalkSpeed` 400.0 (`self.CharacterMovement`))
    (`|AIMoveTo` self (0.0 0.0 0.0) (`GameplayStatics.GetPlayerController` 0)
      (:`OnSuccess`
        (`self.AttackPlayer`))
      (:`OnFail`
        (`self.HunterPlayer`)))))

(event `AttackPlayer`
  (`self.HunterPlayer`))

(event `self.PawnSensing1.OnSeePawn`
  (params (Pawn :type "Pawn Object Reference"))
  (if (not (`self.IsDead`))
    (cast `/Game/ShootingPawn/Blueprints/FPSPlayer_BP` Pawn)
    (set `self.IsActive` true)
    (`self.HunterPlayer`)))

(event `self.PawnSensing1.OnHearNoise`
  (params (Instigator :type "Pawn Object Reference") (Location :type "Vector Structure (by ref)") (Volume :type "Float (single-precision)"))
  (if (not (`self.IsDead`))
    (cast `/Game/ShootingPawn/Blueprints/FPSPlayer_BP` Instigator)
    (set `self.IsActive` true)
    (`self.HunterPlayer`)))

(fn `UserConstructionScript`
  (`parent.UserConstructionScript`))