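; MainMenuMode_BP is the main menu game mode that shows the menu and handles resource preloading before play.
; On BeginPlay it creates the Mainmenu_WB widget, adds it to the viewport, and switches to game-and-UI input with the mouse cursor shown.
; StartLoadResource calls PreLoadMaterials; AssetsLoadComplete then hides the widget's loading view and enables the start button.
; A Test function also triggers the material preload.
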(event `self.ReceiveBeginPlay`
  (bind _returnvalue (`GameplayStatics.GetPlayerController` 0))
  (`KismetSystemLibrary.PrintString` "Hello1111")
  (bind _returnvalue_2 (`|CreateWidget` "/Game/ShootingPawn/Blueprints/UI/Mainmenu_WB.Mainmenu_WB_C"))
  (bind _output_get (set `self.Mainmenu` _returnvalue_2))
  (`UserWidget.AddToViewport` _output_get 0)
  (`WidgetBlueprintLibrary.SetInputMode_GameAndUIEx` _returnvalue null)
  (set `PlayerController.bShowMouseCursor` true _returnvalue))

(event `StartLoadResource`
  (`self.PreLoadMaterials`))

(event `self.AssetsLoadComplete`
  (`Widget.SetVisibility` (`/Game/ShootingPawn/Blueprints/UI/Mainmenu_WB.LoadingView` (`self.Mainmenu`)) "Hidden")
  (`Widget.SetIsEnabled` (`/Game/ShootingPawn/Blueprints/UI/Mainmenu_WB.StartGameBtn` (`self.Mainmenu`)) true))

(fn `Test`
  (`self.PreLoadMaterials`))

(fn `UserConstructionScript`)